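; AfterImageBP is an afterimage effect actor whose visibility fades through a scalar material parameter.
; The construction script creates a dynamic material instance on the AfterImage component's first slot.
; Init sets the starting alpha and unhides the actor, UpdateAlpha subtracts a given amount while initialized, and Finish hides it and clears the flag.
; It hides rather than destroys itself, so the same actor can be reinitialized.
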(event `Init`
  (params (StartAlphaValue :type "Float (double-precision)"))
  (`MaterialInstanceDynamic.SetScalarParameterValue` (`self._dynamicMateInst`) (`self._paramName`) StartAlphaValue)
  (if (`self.bHidden`)
    (`self.SetActorHiddenInGame` false))
  (set `self._initFlag` true))

(event `Finish`
  (`self.SetActorHiddenInGame` true)
  (set `self._initFlag` false))

(event `UpdateAlpha`
  (params (SubValue :type "Float (double-precision)"))
  (bind __dynamicmateinst (`self._dynamicMateInst`))
  (if (`self._initFlag`)
    (bind _returnvalue (`MaterialInstanceDynamic.K2_GetScalarParameterValue` __dynamicmateinst (`self._paramName`)))
    (`MaterialInstanceDynamic.SetScalarParameterValue` __dynamicmateinst (`self._paramName`) (- _returnvalue SubValue))))

(fn `UserConstructionScript`
  (bind _returnvalue (`PrimitiveComponent.CreateDynamicMaterialInstance` (`self.AfterImage`) 0 null "None"))
  (set `self._dynamicMateInst` _returnvalue))
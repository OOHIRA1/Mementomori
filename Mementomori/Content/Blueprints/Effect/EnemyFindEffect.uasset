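; Enemy find effect actor that shows a non-looping Paper2D flipbook attached to an enemy's position.
; On BeginPlay it sets its own lifespan from the enemy's state, lasting longer in the enum's first state than in any other.
; Each Tick it moves itself to the referenced Enemy's location plus an Offset, following by position update without sweep or teleport.
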(event `self.ReceiveBeginPlay`
  (`PaperFlipbookComponent.SetLooping` (`self.FindEffectFlipbook`) false)
  (if (`|EnumEquality` (`/Game/Blueprints/EnemyBP.GetEnemyState` (`self._enemy`)) "NewEnumerator0")
    (`self.SetLifeSpan` 2.5)
    (else
      (`self.SetLifeSpan` 1.5))))

(event `self.ReceiveTick`
  (params (DeltaSeconds :type "Float (single-precision)"))
  (`self.K2_SetActorLocation` (+ (`self.K2_GetActorLocation` (`self._enemy`)) (`self._offset`))))

(fn `UserConstructionScript`)
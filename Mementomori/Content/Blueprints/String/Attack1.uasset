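; Attack1 is a short-lived string effect actor that displays the Effect_word_attack1 word texture.
; On BeginPlay it puts a dynamic instance of StringMaterial_Inst on its String component, sets the Font texture and gives itself a one-second lifespan.
; Each Tick accumulates world delta seconds divided by global time dilation into a timer that drives the material's Time parameter, so the material timing compensates for slow motion.
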(event `self.ReceiveBeginPlay`
  (bind __fontmaterial (`self._fontMaterial`))
  (bind _returnvalue (`KismetMaterialLibrary.CreateDynamicMaterialInstance` "/Game/Material/StringMaterial_Inst.StringMaterial_Inst"))
  (set `self._fontMaterial` _returnvalue)
  (`PrimitiveComponent.SetMaterial` (`self.String`) 0 __fontmaterial)
  (`MaterialInstanceDynamic.SetTextureParameterValue` __fontmaterial "Font" "/Game/Textures/Hero/Attack1/effect_word_attack1.effect_word_attack1")
  (`self.SetLifeSpan` 1.0))

(event `self.ReceiveTick`
  (params (DeltaSeconds :type "Float (single-precision)"))
  (bind _output_get (set `self._timer` (+ (`self._timer`) (/ (`GameplayStatics.GetWorldDeltaSeconds`) (`GameplayStatics.GetGlobalTimeDilation`)))))
  (`MaterialInstanceDynamic.SetScalarParameterValue` (`self._fontMaterial`) "Time" _output_get))

(fn `UserConstructionScript`)
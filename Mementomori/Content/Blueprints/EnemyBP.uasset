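; Paper2D patrolling enemy that picks its animation from state and facing, and switches to alert when its target is the hero.
; Tick derives walk or standby and facing from velocity, selects front or back flipbooks, and rotates the actor 180 degrees to mirror diagonals.
; A hero target raises walk speed and uses caution animations; otherwise the target is the current patrol point.
; Target, search range and patrol-index functions are exposed for external callers.
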(event EventBeginPlay)

(event Collision|EventActorBeginOverlap
  (params (OtherActor :type Actor%20Object%20Reference)))

(event EventTick
  (params (DeltaSeconds :type Float%20%28single-precision%29))
  (bind _charactermovement (Variables|Character|GetCharacterMovement))
  (bind _velocity (Variables|/Script/Engine.MovementComponent|GetVelocity _charactermovement))
  (bind (_x _y) (Math|Vector|BreakVector _velocity))
  (Utilities|FlowControl|Sequence
    (:then_0
      (CallFunction|UpdateFlipbook)
      (|ReverseProcess) ; テクスチャの反転処理
    )
    (:then_1
      (Utilities|Casting|CastToHeroBP (Variables|Default|Get_target)
        (:then
          (Variables|Default|Set_findedPlayerFlag true))
        (:CastFailed
          (Variables|Default|Set_target (Utilities|Array|Get(acopy) (Variables|Default|Get_patrolRoot) (Variables|Default|Get_patrolRootIndex)))))
      (CallFunction|UpdateMaxWalkSpeed))
    (:then_2
      (if (> (Math|Vector|VectorLength (Variables|/Script/Engine.MovementComponent|GetVelocity (Variables|Character|GetCharacterMovement))) 0.0)
        ;[1 1 1] 速度の値から向きを特定し、歩き状態へ
        (Variables|Default|Set_isLookingRight (> _x 0.0))
        (Variables|Default|Set_isLookingForward (< _y 0.0))
        (CallFunction|ChangeEnemyState "NewEnumerator1")
        (else
          ;[1 1 1] キョロキョロしていなかったら待機状態へ
          (if (not (Utilities|Enum|Equal(Enum) (Variables|Default|Get_enemyState) "NewEnumerator2"))
            (CallFunction|ChangeEnemyState "NewEnumerator0")))))))

(fn ConstructionScript)

(fn ChangeEnemyState
  (params (enemyState :type EnemyState%20Enum :default "NewEnumerator0"))
  (Variables|Default|Set_enemyState enemyState))

(fn UpdateFlipbook
  (bind __enemystate (Variables|Default|Get_enemyState))
  (if (Variables|Default|Get_isLookingForward)
    (switch Utilities|FlowControl|Switch|SwitchonEnemyState __enemystate
      (:NewEnumerator0
        (LocalVariables|Setflipbook "/Game/Flipbooks/Enemy/enemy_standby_back_roop_128X128_20.enemy_standby_back_roop_128X128_20"))
      (:NewEnumerator1
        (if (Variables|Default|Get_findedPlayerFlag)
          (LocalVariables|Setflipbook "/Game/Flipbooks/Enemy/enemy_walk_back_caution_128X128_31.enemy_walk_back_caution_128X128_31")
          (else
            (LocalVariables|Setflipbook "/Game/Flipbooks/Enemy/enemy_walk_back_128X128_30.enemy_walk_back_128X128_30"))))
      (:NewEnumerator2
        (LocalVariables|Setflipbook "/Game/Flipbooks/Enemy/enemy_swing_back_128X128_100.enemy_swing_back_128X128_100"))
      (:NewEnumerator3
        (LocalVariables|Setflipbook "/Game/Flipbooks/Enemy/enemy_hit_back_128X128_10.enemy_hit_back_128X128_10"))
      (:NewEnumerator5
        (LocalVariables|Setflipbook "/Game/Flipbooks/Enemy/enemy_KMhit_back_128X128_1.enemy_KMhit_back_128X128_1"))
      (:NewEnumerator4
        (LocalVariables|Setflipbook "/Game/Flipbooks/Enemy/enemy_swoon_intro_back_128X128_10.enemy_swoon_intro_back_128X128_10")))
    (else
      (switch Utilities|FlowControl|Switch|SwitchonEnemyState __enemystate
        (:NewEnumerator0
          (LocalVariables|Setflipbook "/Game/Flipbooks/Enemy/enemy_standby_front_roop_128X128_20.enemy_standby_front_roop_128X128_20"))
        (:NewEnumerator1
          (if (Variables|Default|Get_findedPlayerFlag)
            (LocalVariables|Setflipbook "/Game/Flipbooks/Enemy/enemy_walk_front_roop_caution_128X128_31.enemy_walk_front_roop_caution_128X128_31")
            (else
              (LocalVariables|Setflipbook "/Game/Flipbooks/Enemy/enemy_walk_front_roop_128X128_30.enemy_walk_front_roop_128X128_30"))))
        (:NewEnumerator2
          (LocalVariables|Setflipbook "/Game/Flipbooks/Enemy/enemy_swing_front_128X128_100.enemy_swing_front_128X128_100"))
        (:NewEnumerator3
          (LocalVariables|Setflipbook "/Game/Flipbooks/Enemy/enemy_hit_front_128X128_10.enemy_hit_front_128X128_10"))
        (:NewEnumerator5
          (LocalVariables|Setflipbook "/Game/Flipbooks/Enemy/enemy_KMhit_front_128X128_1.enemy_KMhit_front_128X128_1"))
        (:NewEnumerator4
          (LocalVariables|Setflipbook "/Game/Flipbooks/Enemy/enemy_swoon_intro_front_128X128_10.enemy_swoon_intro_front_128X128_10")))))
  (Sprite|SetFlipbook (Variables|Default|GetSprite) (LocalVariables|Getflipbook)))

(fn GetSearchRange
  (return (Variables|Default|Get_searchRange)))

(fn GetTargetActor
  (return (Variables|Default|Get_target)))

(fn SetTarget
  (params (target :type Actor%20Object%20Reference))
  (Variables|Default|Set_target target))

(fn UpdateMaxWalkSpeed
  (if (Variables|Default|Get_findedPlayerFlag)
    (Variables|/Script/Engine.CharacterMovementComponent|SetMaxWalkSpeed (Variables|Character|GetCharacterMovement) 3.6e+02)
    (else
      (Variables|/Script/Engine.CharacterMovementComponent|SetMaxWalkSpeed (Variables|Character|GetCharacterMovement) 1.5e+02))))

(fn UpdatePatrolRootIndex
  (Variables|Default|Set_patrolRootIndex (|((A+1)%B) (Variables|Default|Get_patrolRootIndex) (Utilities|Array|Length (Variables|Default|Get_patrolRoot)))))
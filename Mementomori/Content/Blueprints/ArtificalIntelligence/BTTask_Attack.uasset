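; Behavior tree task that makes an EnemyBP attack its target, then sets a point to fall back to.
; On execute it caches the pawn; Tick calls Attack if the target is within attack range plus tolerance, otherwise finishes successfully at once.
; After an AttackTime delay, it writes TargetPoint to the blackboard at attack-ready range from the target on the enemy's side, then finishes.
; An animation-state change is left unconnected.
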(event `self.ReceiveExecuteAI`
  (params (OwnerController :type "AIController Object Reference") (ControlledPawn :type "Pawn Object Reference"))
  (bind _asenemy_bp (cast `/Game/Blueprints/EnemyBP` ControlledPawn))
  (set `self._enemy` _asenemy_bp))

(event `self.ReceiveTick`
  (params (OwnerActor :type "Actor Object Reference") (DeltaSeconds :type "Float (single-precision)"))
  (bind __enemy (`self._enemy`))
  (bind __enemy_2 (`self._enemy`))
  (bind _returnvalue (`Actor.K2_GetActorLocation` (`/Game/Blueprints/EnemyBP.GetTarget` (`self._enemy`))))
  (if (<= (`KismetMathLibrary.VSize` (- (`Actor.K2_GetActorLocation` (`/Game/Blueprints/EnemyBP.GetTarget` __enemy)) (`Actor.K2_GetActorLocation` __enemy))) (+ (`/Game/Blueprints/EnemyBP.GetAttackRange` (`self._enemy`)) (`self._tolerance`)))
    (`/Game/Blueprints/EnemyBP.Attack` (`self._enemy`))
    (`KismetSystemLibrary.Delay` (`self._attackTime`))
    (`BTFunctionLibrary.SetBlackboardValueAsVector` (`self._targetPoint`) (+ _returnvalue (* (`KismetMathLibrary.Normal` (- _returnvalue (`Actor.K2_GetActorLocation` __enemy_2))) (* (`/Game/Blueprints/EnemyBP.GetAttackReadyRange` __enemy_2) -1.0)))) ; 攻撃準備範囲上の座標を目的地とする(退く用)
    (`self.FinishExecute` true)
    (else
      (`self.FinishExecute` true) ; 何もせずに完了とする
    )))
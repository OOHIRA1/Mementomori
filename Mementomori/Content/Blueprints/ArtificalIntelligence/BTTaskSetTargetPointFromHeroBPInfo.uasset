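; Behavior tree task that gives an enemy a move destination based on its current HeroBP target.
; Execute caches the controlled EnemyBP, then Tick writes the hero and a TargetPoint to the Blackboard and succeeds, or fails without a hero target.
; The point sits half the attack range short of the hero, on the enemy's side.
; An unfinished angled sidestep approach remains as unconnected nodes.
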(event `self.ReceiveExecuteAI`
  (params (OwnerController :type "AIController Object Reference") (ControlledPawn :type "Pawn Object Reference"))
  (bind _asenemy_bp (cast `/Game/Blueprints/EnemyBP` ControlledPawn))
  (set `self._enemy` _asenemy_bp))

(event `self.ReceiveTick`
  (params (OwnerActor :type "Actor Object Reference") (DeltaSeconds :type "Float (single-precision)"))
  (bind __enemy (`self._enemy`))
  (bind _returnvalue (`Actor.K2_GetActorLocation` (`self._target`)))
  (bind _ashero_bp (cast `/Game/Blueprints/HeroBP` (`/Game/Blueprints/EnemyBP.GetTarget` (`self._enemy`)))
    (:`then`
      (bind _output_get (set `self._target` _ashero_bp))
      (`BTFunctionLibrary.SetBlackboardValueAsObject` (`self._heroBP`) _output_get)
      (`BTFunctionLibrary.SetBlackboardValueAsVector` (`self._targetPoint`) (+ _returnvalue (* (`KismetMathLibrary.Normal` (- _returnvalue (`Actor.K2_GetActorLocation` __enemy))) (* (/ (`/Game/Blueprints/EnemyBP.GetAttackRange` __enemy) 2.0) -1.0)))) ; 攻撃範囲内の座標を目的地とする
      (`self.FinishExecute` true))
    (:`CastFailed`
      (`self.FinishExecute` false))))

(fn `SetPlayerPoint`
  (params (point :type "Vector Structure")))
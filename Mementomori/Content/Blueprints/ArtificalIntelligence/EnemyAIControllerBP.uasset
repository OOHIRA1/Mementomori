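; AI controller for enemy pawns that runs the EnemyLancerBT behavior tree from BeginPlay.
; Every tick it stops the brain logic while the pawn is dead, in a specific animation state (noted as the spotted animation) or handling a hit event.
; A reset DoOnce restarts the logic once when those conditions clear.
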(event `self.ReceiveBeginPlay`
  (`self.RunBehaviorTree` "/Game/Blueprints/ArtificalIntelligence/EnemyLancerBT.EnemyLancerBT"))

(event `self.ReceiveTick`
  (params (DeltaSeconds :type "Float (single-precision)"))
  (if (or (or (`/Game/Blueprints/HealthBP.IsDead` (`self.GetComponentByClass` (`self.K2_GetPawn`) "/Game/Blueprints/HealthBP.HealthBP_C")) (`|EnumEquality` (`/Game/Blueprints/EnemyBP.GetEnemyAnimationState` (cast `/Game/Blueprints/EnemyBP` (`self.K2_GetPawn`) :!pure true)) "NewEnumerator6")) (`/Game/Blueprints/EnemyBP.GetIsStartingHitEvent` (cast `/Game/Blueprints/EnemyBP` (`self.K2_GetPawn`) :!pure true)))
    (`BrainComponent.StopLogic` (`self.BrainComponent`) "")
    (goto _label :!via `Reset`)
    (else
      (`/Engine/EditorBlueprintResources/StandardMacros.DoOnce` true :!label _label
        (:`Completed`
          (`BrainComponent.RestartLogic` (`self.BrainComponent`)))))))

(fn `UserConstructionScript`)
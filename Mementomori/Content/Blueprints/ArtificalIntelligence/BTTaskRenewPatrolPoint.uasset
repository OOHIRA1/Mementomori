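; Behavior tree task that renews an EnemyBP's patrol destination, caching the pawn on execute and doing the work on AI tick.
; It fails if the enemy has no target; within TaskSuccessRange of it, it advances the patrol route index and delays briefly for the target update.
; It then writes the target's location to the TargetPoint blackboard key, prints the target's name and finishes successfully.
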(event `self.ReceiveExecuteAI`
  (params (OwnerController :type "AIController Object Reference") (ControlledPawn :type "Pawn Object Reference"))
  (bind _asenemy_bp (cast `/Game/Blueprints/EnemyBP` ControlledPawn))
  (set `self._enemy` _asenemy_bp))

(event `self.ReceiveTickAI`
  (params (OwnerController :type "AIController Object Reference") (ControlledPawn :type "Pawn Object Reference") (DeltaSeconds :type "Float (single-precision)"))
  (bind _target (`/Game/Blueprints/EnemyBP.GetTarget` (`self._enemy`)))
  ;[1 1 1] 巡回ポイントがあるかの確認
  (if (== (`/Game/Blueprints/EnemyBP.GetTarget` (`self._enemy`)) null)
    (`self.FinishExecute` false)
    (else
      (if (<= (`KismetMathLibrary.VSize` (- (`Actor.K2_GetActorLocation` (`/Game/Blueprints/EnemyBP.GetTarget` (`self._enemy`))) (`Actor.K2_GetActorLocation` ControlledPawn))) (`self._taskSuccessRange`))
        (`/Game/Blueprints/EnemyBP.UpdatePatrolRootIndex` (`self._enemy`))
        (`KismetSystemLibrary.Delay` 1.0) ; Targetの更新を待つ
      )
      (`BTFunctionLibrary.SetBlackboardValueAsVector` (`self._targetPoint`) (`Actor.K2_GetActorLocation` _target))
      (`KismetSystemLibrary.PrintString` (`KismetSystemLibrary.GetDisplayName` _target))
      (`self.FinishExecute` true))))
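; Behavior tree task that feeds an enemy's current patrol target location to the blackboard.
; On AI tick it measures the pawn's distance to the EnemyBP target actor, advancing the patrol root index when within a small radius.
; Otherwise it writes the target's location to TargetKey and finishes successfully.
; Execute and SetPlayerPoint are empty, and a HeroBP range search is left disconnected.
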(event `self.ReceiveExecute`
  (params (OwnerActor :type "Actor Object Reference")))

(event `self.ReceiveTickAI`
  (params (OwnerController :type "AIController Object Reference") (ControlledPawn :type "Pawn Object Reference") (DeltaSeconds :type "Float (single-precision)"))
  (bind _returnvalue (`Actor.K2_GetActorLocation` (`/Game/Blueprints/EnemyBP.GetTargetActor` (`self._enemyBP`))))
  (bind _asenemy_bp (cast `/Game/Blueprints/EnemyBP` ControlledPawn))
  (set `self._enemyBP` _asenemy_bp)
  (if (<= (`KismetMathLibrary.VSize` (- _returnvalue (`Actor.K2_GetActorLocation` ControlledPawn))) 50.0)
    (`/Game/Blueprints/EnemyBP.UpdatePatrolRootIndex` (`self._enemyBP`))
    (else
      (`BTFunctionLibrary.SetBlackboardValueAsVector` (`self._targetKey`) _returnvalue)
      (`self.FinishExecute` true))))

(fn `SetPlayerPoint`
  (params (point :type "Vector Structure")))
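; Behavior Tree task that makes a patrolling EnemyBP perform the action tied to its current patrol point.
; On execute it caches the controlled enemy, then on tick switches on the first tag of the enemy's target.
; Swing Point and Standby Point tags each set an animation state, then share a delay of ActionTime before succeeding.
; Any other tag fails the task immediately.
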(event `self.ReceiveExecuteAI`
  (params (OwnerController :type "AIController Object Reference") (ControlledPawn :type "Pawn Object Reference"))
  (bind _asenemy_bp (cast `/Game/Blueprints/EnemyBP` ControlledPawn))
  (set `self._enemy` _asenemy_bp))

(event `self.ReceiveTick`
  (params (OwnerActor :type "Actor Object Reference") (DeltaSeconds :type "Float (single-precision)"))
  (switch `string` (`KismetStringLibrary.Conv_NameToString` (`|GetArrayItem` (`Actor.Tags` (`/Game/Blueprints/EnemyBP.GetTarget` (`self._enemy`)))))
    (:`Default`
      (`self.FinishExecute` false))
    (:`SwingPoint`
      (`/Game/Blueprints/EnemyBP.ChangeEnemyAnimationState` (`self._enemy`) "NewEnumerator2")
      (`KismetSystemLibrary.Delay` (`self._actionTime`) :!label _label)
      (`self.FinishExecute` true))
    (:`StandbyPoint`
      (`/Game/Blueprints/EnemyBP.ChangeEnemyAnimationState` (`self._enemy`) "NewEnumerator0")
      (goto _label))))
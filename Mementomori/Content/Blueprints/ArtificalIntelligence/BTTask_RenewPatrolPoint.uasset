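; Behavior Tree task that refreshes the patrol destination of an EnemyBP pawn.
; On the AI tick event it fails if the enemy has no patrol target.
; When the pawn is within TaskSuccessRange of the target, it advances the enemy's patrol route index.
; It then writes the current target's location to the TargetPoint blackboard key and finishes successfully.
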(event `self.ReceiveTickAI`
  (params (OwnerController :type "AIController Object Reference") (ControlledPawn :type "Pawn Object Reference") (DeltaSeconds :type "Float (single-precision)"))
  (bind _asenemy_bp (cast `/Game/Blueprints/EnemyBP` ControlledPawn))
  (set `self._enemy` _asenemy_bp)
  ;[1 1 1] 巡回ポイントがあるかの確認
  (if (== (`/Game/Blueprints/EnemyBP.GetTarget` (`self._enemy`)) null)
    (`self.FinishExecute` false)
    (else
      (if (<= (`KismetMathLibrary.VSize` (- (`Actor.K2_GetActorLocation` (`/Game/Blueprints/EnemyBP.GetTarget` (`self._enemy`))) (`Actor.K2_GetActorLocation` ControlledPawn))) (`self._taskSuccessRange`))
        (`/Game/Blueprints/EnemyBP.UpdatePatrolRootIndex` (`self._enemy`)))
      (`BTFunctionLibrary.SetBlackboardValueAsVector` (`self._targetPoint`) (`Actor.K2_GetActorLocation` (`/Game/Blueprints/EnemyBP.GetTarget` (`self._enemy`))))
      (`self.FinishExecute` true))))
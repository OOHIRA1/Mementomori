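; TalkManagerBP manages paged talk-event dialogue loaded from a Data Table.
; Generate copies each row into the Data array, counts pages, then creates the TalkWidget and adds it to the viewport.
; FlipPage advances the page within bounds and is the only step that sets PageData, which GetText reads for its text.
; Missing data and page overruns print on-screen errors through PrintError.
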(event `self.ReceiveBeginPlay`)

(fn `createUI`
  (bind _returnvalue (`|CreateWidget` "/Game/Blueprints/TalkEvent/TalkWidget.TalkWidget_C"))
  (set `self.UI` _returnvalue)
  (`UserWidget.AddToViewport` _returnvalue 0)
  (return))

(fn `flipPage`
  (bind _exist (`self.isExistData`))
  (if _exist
    (bind _result (`/Engine/EditorBlueprintResources/StandardMacros.IncrementInt` (`self.page`))
      (:`  `
        (if (< _result (`self.maxPage`))
          (bind _output_get (set `self.page` _result))
          (`KismetSystemLibrary.PrintString` (`KismetStringLibrary.Concat_StrStr` "Page : " (`KismetStringLibrary.Conv_IntToString` _output_get)))
          (set `self.pageData` (`|GetArrayItem` (`self.data`) _output_get))
          (else
            (`self.printError` (`self.ERROR_PAGE_OVER`))))))
    (else
      (`self.printError` (`self.ERROR_NOT_EXIST`))))
  (return))

(fn `generate`
  (params (targetType :type "DataTable Object Reference"))
  (bind _outrownames (`DataTableFunctionLibrary.GetDataTableRowNames` targetType))
  (for (_array_element _array_index) _outrownames
    (bind _returnvalue (`|GetDataTableRow` targetType _array_element)
      (:`then`
        (`KismetArrayLibrary.Array_Set` (`self.data`) _array_index _returnvalue true)
        ;[1 1 1] 最大ページ数を更新
        (bind _result (`/Engine/EditorBlueprintResources/StandardMacros.IncrementInt` (`self.maxPage`))
          (:`  `
            (set `self.maxPage` _result))))))
  (bind _exist (`self.isExistData`))
  (if _exist
    (`KismetSystemLibrary.PrintString` "Complete Load TalkData" true true (struct :`G` 1.0 :`B` 0.179893 :`A` 1.0))
    (`self.createUI`)
    (else
      (`self.printError` (`self.ERROR_NOT_EXIST`))))
  (return))

(fn `getText`
  (returns (returnText :type String))
  (locals (text :type String))
  (bind _exist (`self.isExistData`))
  (if _exist
    (set `local.text` (`.Text_21_3243275B4B15F5115C8EE38DC3E4CAC6` (break `/Game/Blueprints/Struct/TalkData` (`self.pageData`))))
    (else
      (`self.printError` (`self.ERROR_NOT_EXIST`))
      (set `local.text` "NONE")))
  (return (`local.text`)))

(fn `isExistData`
  (returns (exist :type Boolean))
  (return (> (`self.maxPage`) 0)))

(fn `printError`
  (params (message :type String))
  (`KismetSystemLibrary.PrintString` (`KismetStringLibrary.Concat_StrStr` "<<< ERROR >>>" message) true true (struct :`R` 255.0 :`A` 1.0) 5.0)
  (return))

(fn `UserConstructionScript`)
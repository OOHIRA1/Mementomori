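; TalkDataBP holds the page data for a talk event and tracks the page currently shown.
; Initialize stores the page array and shows the first page, and FlipPage advances until the last one.
; Each update converts the page text and resolves body, face and two effect illustrations for four screen positions through DataAsset lookups.
; GetText and GetIllust expose the current text and per-position illustration parts.
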(fn `flipPage`
  (bind _result (`self.isPageMax`))
  (if _result
    (return)
    (else
      (bind _result_2 (`/Engine/EditorBlueprintResources/StandardMacros.IncrementInt` (`self._pageNum`))
        (:`  `
          (bind _output_get (set `self._pageNum` _result_2))
          (set `self._showPage` (`|GetArrayItem` (`self._allPage`) _output_get))
          (`self.update`))))))

(fn `getIllust`
  (params (Pos :type "/Game/Blueprints/Enum/TalkerPos Enum" :default "NewEnumerator0") (Parts :type "/Game/Blueprints/Enum/TalkerParts Enum" :default "NewEnumerator0"))
  (returns (result :type "Object Object Reference"))
  (locals (_result :type "Object Object Reference"))
  (bind (_value _returnvalue) (`BlueprintMapLibrary.Map_Find` (`self._talkerData`) Pos))
  (bind (_bodyillust _faceillust _effectparts1 _effectparts2) (break `/Game/Blueprints/Struct/TalkEvent/TalkerDataBase` _value))
  (if _returnvalue
    (switch `/Game/Blueprints/Enum/TalkerParts` Parts
      (:`NewEnumerator0`
        (set `local._result` _bodyillust))
      (:`NewEnumerator1`
        (set `local._result` _faceillust))
      (:`NewEnumerator2`
        (set `local._result` _effectparts1))
      (:`NewEnumerator3`
        (set `local._result` _effectparts2)))
    (return (`local._result`))))

(fn `getText`
  (returns (text :type Text))
  (return (`self._text`)))

(fn `initialize`
  (params (talkData :type "Array of /Game/Blueprints/Struct/TalkEvent/TalkData Structure"))
  ;[1 1 1] 変数の初期
  (bind _output_get (set `self._allPage` talkData))
  (set `self._showPage` (`|GetArrayItem` _output_get))
  (set `self._pageNum` 0)
  (set `self._maxPageNum` (`KismetArrayLibrary.Array_Length` _output_get))
  (`self.update`))

(fn `isPageMax`
  (returns (result :type Boolean))
  (return (>= (`self._pageNum`) (- (`self._maxPageNum`) 1))))

(fn `update`
  (`self.updateText`)
  (`self.updateIllust`))

(fn `updateIllust`
  (locals (LeftLeft :type "/Game/Blueprints/Enum/TalkerPos Enum") (Left :type "/Game/Blueprints/Enum/TalkerPos Enum" :default "NewEnumerator1") (RightRight :type "/Game/Blueprints/Enum/TalkerPos Enum" :default "NewEnumerator2") (Right :type "/Game/Blueprints/Enum/TalkerPos Enum" :default "NewEnumerator3"))
  (bind __talkerdata (`self._talkerData`))
  (bind (_illust_left_left _illust_left _illust_right_right _illust_right _illust_talker _label_talker _text _faceparts_left_left _faceparts_left _faceparts_right_right _faceparts_right _effectparts_1_left_left _effectparts_1_left _effectparts_1_right_right _effectparts_1_right _effectparts_2_left_left _effectparts_2_left _effectparts_2_right_right _effectparts_2_right) (break `/Game/Blueprints/Struct/TalkEvent/TalkData` (`self._showPage`)))
  (bind __assetdata (`/Game/Blueprints/TalkEvent/DABase/TalkIllustDABase._assetData` (`self._dataAsset`)))
  (`BlueprintMapLibrary.Map_Add` __talkerdata (`local.LeftLeft`) (make `/Game/Blueprints/Struct/TalkEvent/TalkerDataBase` (`BlueprintMapLibrary.Map_Find` __assetdata _illust_left_left) (`BlueprintMapLibrary.Map_Find` __assetdata _faceparts_left_left) (`BlueprintMapLibrary.Map_Find` __assetdata _effectparts_1_left_left) (`BlueprintMapLibrary.Map_Find` __assetdata _effectparts_2_left_left)))
  (`BlueprintMapLibrary.Map_Add` __talkerdata (`local.Left`) (make `/Game/Blueprints/Struct/TalkEvent/TalkerDataBase` (`BlueprintMapLibrary.Map_Find` __assetdata _illust_left) (`BlueprintMapLibrary.Map_Find` __assetdata _faceparts_left) (`BlueprintMapLibrary.Map_Find` __assetdata _effectparts_1_left) (`BlueprintMapLibrary.Map_Find` __assetdata _effectparts_2_left)))
  (`BlueprintMapLibrary.Map_Add` __talkerdata (`local.RightRight`) (make `/Game/Blueprints/Struct/TalkEvent/TalkerDataBase` (`BlueprintMapLibrary.Map_Find` __assetdata _illust_right_right) (`BlueprintMapLibrary.Map_Find` __assetdata _faceparts_right_right) (`BlueprintMapLibrary.Map_Find` __assetdata _effectparts_1_right_right) (`BlueprintMapLibrary.Map_Find` __assetdata _effectparts_2_right_right)))
  (`BlueprintMapLibrary.Map_Add` __talkerdata (`local.Right`) (make `/Game/Blueprints/Struct/TalkEvent/TalkerDataBase` (`BlueprintMapLibrary.Map_Find` __assetdata _illust_right) (`BlueprintMapLibrary.Map_Find` __assetdata _faceparts_right) (`BlueprintMapLibrary.Map_Find` __assetdata _effectparts_1_right) (`BlueprintMapLibrary.Map_Find` __assetdata _effectparts_2_right))))

(fn `updateText`
  (set `self._text` (`KismetTextLibrary.Conv_StringToText` (`.Text_21_3243275B4B15F5115C8EE38DC3E4CAC6` (break `/Game/Blueprints/Struct/TalkEvent/TalkData` (`self._showPage`))))))

(fn `UserConstructionScript`)
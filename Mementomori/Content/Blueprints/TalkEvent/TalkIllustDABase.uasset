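; Data asset base for talk event illustrations, holding a map of assets keyed by asset name.
; Load clears the map through Initialize, which also prints a debug message, then scans the configured Path recursively through the Asset Registry.
; Each asset found is resolved with GetAsset and added under its name, so the map fills from folder contents.
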(fn `Initialize`
  (`BlueprintMapLibrary.Map_Clear` (`self._assetData`))
  (`KismetSystemLibrary.PrintString` null "Clear Complete < TalkIllustDA >" true true (struct :`G` 0.66 :`B` 1.0 :`A` 1.0) 3.0)
  (return))

(fn `Load`
  (locals (NewLocalVar_0 :type Integer))
  (`self.Initialize`)
  (for _array_element (`AssetRegistry.GetAssetsByPath` (`AssetRegistryHelpers.GetAssetRegistry`) (`KismetStringLibrary.Conv_StringToName` (`self._path`)) true false)
    (`BlueprintMapLibrary.Map_Add` (`self._assetData`) (`KismetStringLibrary.Conv_NameToString` (`.AssetName` (break `AssetData` _array_element))) (`AssetRegistryHelpers.GetAsset` _array_element))))
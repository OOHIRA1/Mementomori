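; UIHUDBP is the HUD Blueprint that creates and displays the player's gameplay UI widgets.
; On BeginPlay it adds the HP gauge, item gauge, mission start and combo hit widgets to the viewport.
; Each Tick it polls the HeroBP player mode and, on KM INTRO, uses a DoOnce to add the KMCutInBP cut-in widget a single time.
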(event `self.ReceiveBeginPlay`
  (`|ExecutionSequence`
    (:`then_0`
      (bind _returnvalue (`|CreateWidget` "/Game/Blueprints/Widget/HPGaugeBP.HPGaugeBP_C"))
      (`UserWidget.AddToViewport` _returnvalue 0))
    (:`then_1`
      (bind _returnvalue_2 (`|CreateWidget` "/Game/Blueprints/Widget/WD_ItemGauge.WD_ItemGauge_C"))
      (`UserWidget.AddToViewport` _returnvalue_2 0))
    (:`then_2`
      (bind _returnvalue_3 (`|CreateWidget` "/Game/Blueprints/Widget/WD_MissionStart.WD_MissionStart_C"))
      (`UserWidget.AddToViewport` _returnvalue_3 0))
    (:`then_3`
      (bind _returnvalue_4 (`|CreateWidget` "/Game/Blueprints/Widget/WD_ComboHit.WD_ComboHit_C"))
      (`UserWidget.AddToViewport` _returnvalue_4 0))))

(event `self.ReceiveTick`
  (params (DeltaSeconds :type "Float (single-precision)"))
  (bind _ashero_bp (cast `/Game/Blueprints/HeroBP` (`GameplayStatics.GetPlayerCharacter` 0)))
  (bind _playermode (`/Game/Blueprints/HeroBP.GetPlayerMode` _ashero_bp))
  (switch `/Game/Blueprints/Enum/HeroMode` _playermode
    (:`NewEnumerator1`
      (`/Engine/EditorBlueprintResources/StandardMacros.DoOnce` false
        (:`Completed`
          (bind _returnvalue (`|CreateWidget` "/Game/Blueprints/Widget/KMCutInBP.KMCutInBP_C"))
          (`UserWidget.AddToViewport` _returnvalue 0))))))

(fn `UserConstructionScript`)
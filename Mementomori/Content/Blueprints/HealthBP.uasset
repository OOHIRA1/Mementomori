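; HealthBP is a health container that stores a Health value and exposes functions to set, read, damage and test it for death.
; ChangeHealth accepts values only between zero and MAXHEALTH, while Damage subtracts points and floors the result at zero.
; IsDead reports true once Health reaches zero or below.
; The event graph has no active logic, so any change comes through function calls.
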(fn `ChangeHealth`
  (params (health :type "Float (double-precision)"))
  (if (and (>= health 0.0) (<= health (`self.MAX_HEALTH`)))
    (set `self._health` health))
  (return))

(fn `Damage`
  (params (damagePoint :type "Float (double-precision)"))
  (bind _returnvalue (- (`self._health`) damagePoint))
  (if (<= _returnvalue 0.0)
    (set `self._health` 0.0)
    (else
      (set `self._health` _returnvalue))))

(fn `GetHealth`
  (returns (health :type "Float (double-precision)"))
  (return (`self._health`)))

(fn `IsDead`
  (returns (dead :type Boolean))
  (return (<= (`self._health`) 0.0)))
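; Field-of-view helper Blueprint that tracks which actors of target classes are inside its detection sphere.
; SphereCollision begin overlap adds an actor to DetectedActors if its exact class is listed in TargetActors, and end overlap removes it.
; GetDetectedActors exposes the list; detection relies purely on overlap, with no angle or line-of-sight checks.
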(event `self.SphereCollision.OnComponentBeginOverlap`
  (params (OverlappedComponent :type "PrimitiveComponent Object Reference") (OtherActor :type "Actor Object Reference") (OtherComp :type "PrimitiveComponent Object Reference") (OtherBodyIndex :type Integer) (bFromSweep :type Boolean) (SweepResult :type "HitResult Structure (by ref)"))
  ;[1 1 1] 視野に入った時の処理
  (if (`KismetArrayLibrary.Array_Contains` (`self._targetActors`) (`GameplayStatics.GetObjectClass` OtherActor))
    (`KismetArrayLibrary.Array_AddUnique` (`self._detectedActors`) OtherActor)))

(event `self.SphereCollision.OnComponentEndOverlap`
  (params (OverlappedComponent :type "PrimitiveComponent Object Reference") (OtherActor :type "Actor Object Reference") (OtherComp :type "PrimitiveComponent Object Reference") (OtherBodyIndex :type Integer))
  (bind _returnvalue (`KismetArrayLibrary.Array_Find` (`self._detectedActors`) OtherActor))
  ;[1 1 1] 視野外に出た時の処理
  (if (>= _returnvalue 0)
    (`KismetArrayLibrary.Array_Remove` (`self._detectedActors`) _returnvalue)))

(fn `GetDetectedActors`
  (returns (detectedActors :type "Array of Actor Object Reference"))
  (return (`self._detectedActors`)))

(fn `UserConstructionScript`)
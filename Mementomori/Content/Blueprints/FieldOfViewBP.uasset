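; FieldOfViewBP is a field-of-view sensor that tracks which actors are inside its Cone component.
; An actor that begins overlapping the cone is added uniquely to the ViewActors array.
; When an overlap ends, a loop over the array removes the matching entry by index.
; GetViewActors returns the current array, and detection relies solely on overlap events, with no Tick logic.
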(event `self.ReceiveTick`
  (params (DeltaSeconds :type "Float (single-precision)")))

(event `self.Cone.OnComponentBeginOverlap`
  (params (OverlappedComponent :type "PrimitiveComponent Object Reference") (OtherActor :type "Actor Object Reference") (OtherComp :type "PrimitiveComponent Object Reference") (OtherBodyIndex :type Integer) (bFromSweep :type Boolean) (SweepResult :type "HitResult Structure (by ref)"))
  ;[1 1 1] 視野に入った時の処理
  (`KismetArrayLibrary.Array_AddUnique` (`self._viewActors`) OtherActor))

(event `self.Cone.OnComponentEndOverlap`
  (params (OverlappedComponent :type "PrimitiveComponent Object Reference") (OtherActor :type "Actor Object Reference") (OtherComp :type "PrimitiveComponent Object Reference") (OtherBodyIndex :type Integer))
  ;[1 1 1] 視野外に出た時の処理
  (for (_array_element _array_index) (`self._viewActors`)
    (if (== _array_element OtherActor)
      (`KismetArrayLibrary.Array_Remove` (`self._viewActors`) _array_index))))

(fn `GetViewActors`
  (returns (viewActors :type "Array of Actor Object Reference"))
  (return (`self._viewActors`)))

(fn `UserConstructionScript`)